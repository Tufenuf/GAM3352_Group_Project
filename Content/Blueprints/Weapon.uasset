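; Weapon Blueprint that spawns a Projectile at ProjectileSpawnPoint, with firing gated by trigger state and RoundsPerSecond.
; PullTrigger passes a DoOnce to fire immediately, set a named timer for Fire one interval later, and hold IsReloading for that interval.
; ReleaseTrigger clears the timer and resets the DoOnce, while IsReloading still blocks re-pulls until the delay ends, preventing faster fire through repeated presses.
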(event `PullTrigger`
  (bind _returnvalue (/ 1.0 (`self.RoundsPerSecond`)))
  (if (not (`self.isReloading`))
    (`/Engine/EditorBlueprintResources/StandardMacros.DoOnce` false :!label _label
      (:`Completed`
        (`self.Fire`)
        (`KismetSystemLibrary.K2_SetTimer` null "Fire" _returnvalue)
        (set `self.isReloading` true)
        (`KismetSystemLibrary.Delay` _returnvalue)
        (set `self.isReloading` false)))))

(event `ReleaseTrigger`
  (`KismetSystemLibrary.K2_ClearTimer` null "Fire")
  (goto _label :!via `Reset`))

(event `Fire`
  (`|SpawnActorFromClass` "/Game/Blueprints/Projectile.Projectile_C" (`SceneComponent.K2_GetComponentToWorld` (`self.ProjectileSpawnPoint`)) "Undefined" "OverrideRootScale" null null))

(fn `UserConstructionScript`)