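; BP_Fire is a fire hazard that damages a HeroCharacter standing inside its Box collision.
; Begin overlap sets an IsOverlap flag and starts a Delay-based loop that sends a negative AffectHealthMessage to the hero every second.
; The loop stops once the hero is dead or an end overlap from a HeroCharacter clears the flag.
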(event `self.Box.OnComponentBeginOverlap`
  (params (OverlappedComponent :type "PrimitiveComponent Object Reference") (OtherActor :type "Actor Object Reference") (OtherComp :type "PrimitiveComponent Object Reference") (OtherBodyIndex :type Integer) (bFromSweep :type Boolean) (SweepResult :type "HitResult Structure (by ref)"))
  (set `self.IsOverlap` true)
  (bind _ashero_character (cast `/Game/Blueprints/HeroCharacter` OtherActor))
  (if (`/Game/Blueprints/BaseCharacter.IsDead` _ashero_character) :!label _label
    (set `self.IsOverlap` false)
    (elif (`self.IsOverlap`)
      (message `/Game/Blueprints/iDamagable.AffectHealth` _ashero_character -10.0)
      (`KismetSystemLibrary.Delay` 1.0)
      (goto _label))))

(event `self.Box.OnComponentEndOverlap`
  (params (OverlappedComponent :type "PrimitiveComponent Object Reference") (OtherActor :type "Actor Object Reference") (OtherComp :type "PrimitiveComponent Object Reference") (OtherBodyIndex :type Integer))
  (cast `/Game/Blueprints/HeroCharacter` OtherActor)
  (set `self.IsOverlap` false))

(fn `UserConstructionScript`)