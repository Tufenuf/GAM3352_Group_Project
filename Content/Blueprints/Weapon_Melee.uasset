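; Melee weapon Blueprint that damages damageable actors touched by its hitbox, skipping those tagged Friendly.
; SwingTrigger, gated by a DoOnce, sets a one-shot "Fire" timer based on swing rate; SwingRelease clears and resets it.
; SwingWeapon briefly enables hitbox collision, and overlaps send a fixed health reduction through IDamagable.
; No "Fire" function appears here, and the SwingWeapon call and projectile spawn are disconnected.
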(event `SwingTrigger`
  (`/Engine/EditorBlueprintResources/StandardMacros.DoOnce` false :!label _label
    (:`Completed`
      (`KismetSystemLibrary.K2_SetTimer` null "Fire" (/ 1.0 (`self.SwingsPerSecond`))))))

(event `SwingRelease`
  (`KismetSystemLibrary.K2_ClearTimer` null "Fire")
  (goto _label :!via `Reset`))

(event `SwingWeapon`
  (`PrimitiveComponent.SetCollisionEnabled` (`self.Hitbox`) "QueryAndPhysics")
  (`KismetSystemLibrary.Delay` 0.2)
  (`PrimitiveComponent.SetCollisionEnabled` (`self.Hitbox`) "NoCollision"))

(event `self.Hitbox.OnComponentBeginOverlap`
  (params (OverlappedComponent :type "PrimitiveComponent Object Reference") (OtherActor :type "Actor Object Reference") (OtherComp :type "PrimitiveComponent Object Reference") (OtherBodyIndex :type Integer) (bFromSweep :type Boolean) (SweepResult :type "HitResult Structure (by ref)"))
  (if (`KismetSystemLibrary.DoesImplementInterface` OtherActor "/Game/Blueprints/iDamagable.iDamagable_C")
    (if (not (`self.ActorHasTag` OtherActor "Friendly"))
      (message `/Game/Blueprints/iDamagable.AffectHealth` OtherActor -20.0))))

(fn `UserConstructionScript`)