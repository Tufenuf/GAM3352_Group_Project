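; BaseCharacter is a character Blueprint, named as a base class, that tracks Health and a dead state.
; CalculateHealth adds a signed delta to Health, capped at 100 with no lower clamp, then calls CalculateDead.
; CalculateDead sets IsDead whenever Health is zero or below and clears it otherwise.
; The event graph and construction script hold no logic.
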(fn `CalculateDead`
  (if (<= (`self.Health`) 0.0)
    (set `self.IsDead` true)
    (else
      (set `self.IsDead` false))))

(fn `CalculateHealth`
  (params (Delta :type "Float (double-precision)"))
  (bind _returnvalue (+ (`self.Health`) Delta))
  (if (> _returnvalue 100.0)
    (set `self.Health` 100.0)
    (else
      (set `self.Health` _returnvalue)))
  (`self.CalculateDead`))

(fn `UserConstructionScript`)