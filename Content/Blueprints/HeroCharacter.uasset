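; Player hero character for a twin-stick shooter, handling movement, cooldown-limited dash, gun and melee combat, and death.
; BeginPlay spawns both weapons on GunSocket, hands the spawn transform to TwinStickMode and creates the HUD.
; Look input past a dead zone sets facing and auto-fires while ammo remains; melee input toggles weapon visibility and swings.
; Damage plays a bark; death disables input, then after a delay requests respawn and destroys character, weapons and HUD.
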(event `Event Adjust Ammo`
  (params (Value :type Integer))
  ;[1 1 1] Adjust Ammo Count
  (set `self.AmmoCount` (+ (`self.AmmoCount`) Value))
  (`/Game/Blueprints/WidgetsUI/TwinStickHUD.UpdateAmmo` (`self.PlayerUIRef`) (`self.AmmoCount`)))

(event `self.ReceiveBeginPlay`
  (bind _mesh (`self.Mesh`))
  (bind _mesh_2 (`self.Mesh`))
  (`|ExecutionSequence`
    (:`then_0`
      ;[1 1 1] Weapon Setup
      (bind _returnvalue (`|SpawnActorFromClass` "/Game/Blueprints/Weapon.Weapon_C" (`SceneComponent.K2_GetComponentToWorld` _mesh) "Undefined" "OverrideRootScale" null null))
      (bind _output_get (set `self.Weapon` _returnvalue))
      (`self.K2_AttachToComponent` (`self.Weapon`) _mesh "GunSocket" "SnapToTarget" "SnapToTarget" "KeepWorld" true)
      (`self.K2_AttachToComponent` _output_get _mesh "GunSocket" "SnapToTarget" "SnapToTarget" "KeepWorld" true)
      ;[1 1 1] Melee Setup
      (bind _returnvalue_2 (`|SpawnActorFromClass` "/Game/Blueprints/Weapon_Melee.Weapon_Melee_C" (`SceneComponent.K2_GetComponentToWorld` _mesh_2) "Undefined" "OverrideRootScale" null null))
      (bind _output_get_2 (set `self.Melee` _returnvalue_2))
      (`self.K2_AttachToComponent` _output_get_2 _mesh_2 "GunSocket" "SnapToTarget" "SnapToTarget" "KeepWorld" true)
      (`SceneComponent.ToggleVisibility` (`/Game/Blueprints/Weapon_Melee.MeleeMesh` _output_get_2) false))
    (:`then_1`
      ;[1 1 1] SendSpawnTransformUpToGameMode
      (bind _astwin_stick_mode (cast `/Game/Blueprints/TwinStickMode` (`GameplayStatics.GetGameMode`)))
      (bind _output_get_3 (set `self.GameMode` _astwin_stick_mode))
      (set `/Game/Blueprints/TwinStickMode.PlayerSpawnTransform` (`self.GetTransform`) _output_get_3))
    (:`then_2`
      ;[1 1 1] Player UI HUD Update
      (bind _returnvalue_3 (`|CreateWidget` "/Game/Blueprints/WidgetsUI/TwinStickHUD.TwinStickHUD_C"))
      (bind _output_get_4 (set `self.PlayerUIRef` _returnvalue_3))
      (`UserWidget.AddToViewport` _output_get_4 0)
      (`self.Update Default UI`))
    (:`then_3`
      (set `self.AmmoCount` (`self.AmmoCount`)))))

(event `InputAxis|MoveUp`
  (params (AxisValue :type "Float (single-precision)"))
  ;[1 1 1] Movement
  (`self.AddMovementInput` (1.0 0.0 0.0) AxisValue))

(event `InputAction|Dash`
  (params (Key :type "Key Structure"))
  ;[1 1 1] Dash
  (:`Pressed`
    (if (`self.Dodge`)
      (`self.LaunchCharacter` (* (`SceneComponent.GetForwardVector` (`self.CapsuleComponent`)) 5000.0))
      (set `self.Dodge` false)
      (`KismetSystemLibrary.Delay` 8.0)
      (set `self.Dodge` true))))

(event `InputAxis|MoveRight`
  (params (AxisValue :type "Float (single-precision)"))
  ;[1 1 1] Movement
  (`self.AddMovementInput` (0.0 1.0 0.0) AxisValue))

(event `InputAxis|LookUp`
  (params (AxisValue :type "Float (single-precision)"))
  (bind _weapon (`self.Weapon`))
  ;[1 1 1] Rotation
  (bind _returnvalue (`KismetMathLibrary.MakeVector` AxisValue (stale `InputAxis|LookRight` AxisValue)))
  (if (> (`KismetMathLibrary.VSize` _returnvalue) 0.25) :!label _label
    (`Controller.SetControlRotation` (`self.GetController`) (`KismetMathLibrary.Conv_VectorToRotator` _returnvalue))
    (if (> (`self.AmmoCount`) 0)
      (`KismetSystemLibrary.Delay` 0.001)
      (`/Game/Blueprints/Weapon.PullTrigger` _weapon))
    (else
      (`/Game/Blueprints/Weapon.ReleaseTrigger` _weapon))))

(event `InputAxis|LookRight`
  (params (AxisValue :type "Float (single-precision)"))
  ;[1 1 1] Rotation
  (goto _label))

(event `/Game/Blueprints/iDamagable.AffectHealth`
  (params (Delta :type "Float (single-precision)"))
  (`GameplayStatics.PlaySound2D` "/Game/Audio/SoundCues/SC_HeroBarks.SC_HeroBarks" 1.0 1.0 0.0 null null)
  (`self.CalculateHealth` Delta)
  (`KismetSystemLibrary.PrintString` (`KismetStringLibrary.Conv_DoubleToString` (`self.Health`)))
  (if (`self.IsDead`)
    (`self.DisableInput` null)
    (`KismetSystemLibrary.Delay` 3.0)
    (`/Game/Blueprints/TwinStickMode.RespawnPlayer` (`self.GameMode`))
    (`Widget.RemoveFromParent` (`self.PlayerUIRef`))
    (`self.K2_DestroyActor` (`self.Weapon`))
    (`self.K2_DestroyActor` self)
    (`self.K2_DestroyActor` (`self.Melee`))))

(event `Toggle HUD OFF`
  ;[1 1 1] Pause Menu HUD Toggle
  (`Widget.RemoveFromParent` (`self.PlayerUIRef`)))

(event `Toggle HUD ON`
  ;[1 1 1] Pause Menu HUD Toggle
  (`UserWidget.AddToViewport` (`self.PlayerUIRef`) 0))

(event `InputAction|Melee`
  (params (Key :type "Key Structure"))
  (bind _melee (`self.Melee`))
  (bind _meleemesh (`/Game/Blueprints/Weapon_Melee.MeleeMesh` _melee))
  ;[1 1 1] Melee
  (:`Pressed`
    (`SceneComponent.ToggleVisibility` (`/Game/Blueprints/Weapon.StaticMesh` (`self.Weapon`)) false)
    (`SceneComponent.ToggleVisibility` _meleemesh false)
    (`/Game/Blueprints/Weapon_Melee.SwingWeapon` _melee))
  (:`Released`
    (`/Game/Blueprints/Weapon_Melee.SwingRelease` _melee)
    (`SceneComponent.ToggleVisibility` _meleemesh false)
    (`SceneComponent.ToggleVisibility` (`/Game/Blueprints/Weapon.StaticMesh` (`self.Weapon`)) false)))

(fn `Update Default UI`
  (`/Game/Blueprints/WidgetsUI/TwinStickHUD.UpdateAmmo` (`self.PlayerUIRef`) (`self.AmmoCount`)))

(fn `UserConstructionScript`
  (`parent.UserConstructionScript`))