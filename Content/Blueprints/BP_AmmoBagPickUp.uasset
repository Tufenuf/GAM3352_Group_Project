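; BP_AmmoBagPickUp is an ammo pickup that refills the hero's ammo when touched.
; It adds a rotating movement component on BeginPlay so the bag spins.
; When a HeroCharacter overlaps its collision, it adds AmmoGiven to the hero's AmmoCount and plays a pickup sound.
; It then destroys itself and pushes the new count to the hero's UI, with that update running after the destroy call.
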(event `self.ReceiveBeginPlay`
  (`AddComponent|NODE_AddRotatingMovementComponent-0`))

(event `self.Collision.OnComponentBeginOverlap`
  (params (OverlappedComponent :type "PrimitiveComponent Object Reference") (OtherActor :type "Actor Object Reference") (OtherComp :type "PrimitiveComponent Object Reference") (OtherBodyIndex :type Integer) (bFromSweep :type Boolean) (SweepResult :type "HitResult Structure (by ref)"))
  (bind _ashero_character (cast `/Game/Blueprints/HeroCharacter` OtherActor))
  (bind _output_get (set `/Game/Blueprints/HeroCharacter.AmmoCount` (+ (`/Game/Blueprints/HeroCharacter.AmmoCount` _ashero_character) (`self.AmmoGiven`)) _ashero_character))
  (`GameplayStatics.PlaySound2D` "/Game/Audio/A_AmmoPickup.A_AmmoPickup" 1.0 1.0 0.0 null null)
  (`self.K2_DestroyActor`)
  (`/Game/Blueprints/WidgetsUI/TwinStickHUD.UpdateAmmo` (`/Game/Blueprints/HeroCharacter.PlayerUIRef` _ashero_character) _output_get))

(fn `UserConstructionScript`)